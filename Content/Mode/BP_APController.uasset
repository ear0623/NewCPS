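; BP_APController is a controller that fetches JSON from two hard-coded HTTP API servers at BeginPlay and prints debug output.
; It creates two HTTPObjects, one for a hierarchy request and one for a Type01 main-data request.
; All four progress, completion and JSON callbacks are bound on the hierarchy object only.
; Generated handlers store callback structs and loop over their data, one printing each Type01 DataName.
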(event Custom|OnProceess
  (params (RecvSize :type Integer) (TotalSize :type Integer) (Percent :type Float%20%28single-precision%29))
  ;[1 1 1] HTTP Connect
  (Development|PrintString (Utilities|String|ToString(Text) (Utilities|Text|FormatText "{a}/{b} 는 {P}" RecvSize TotalSize Percent)) true true "(R=1.000000,G=0.095008,B=0.000000,A=1.000000)" 1e+01))

(event Custom|OnFinished
  (params (bIsSuccess :type Boolean) (ContentPath :type String))
  ;[1 1 1] HTTP Connect
  (Development|PrintString (Utilities|String|ToString(Boolean) bIsSuccess) true true "(R=1.000000,G=0.076702,B=0.000000,A=1.000000)" 1e+01)
  (Development|PrintString "Hello"))

(event EventBeginPlay
  ;[1 1 1] HTTP Connect
  (bind _returnvalue (Game|ConstructObjectfromClass "/Script/Project_CPS.HTTPObject"))
  (bind _returnvalue_2 (Game|ConstructObjectfromClass "/Script/Project_CPS.HTTPObject"))
  (Variables|Default|SetMainHTTP _returnvalue_2)
  (Variables|Default|SetBP_HTTPOB _returnvalue)
  (EventDispatchers|BindEventtoOnHttpConnectProcessCallback _returnvalue (EventDispatchers|CreateEvent :!event Custom|OnProceess))
  (EventDispatchers|BindEventtoOnHttpConnectFinishedCallback _returnvalue (EventDispatchers|CreateEvent :!event Custom|OnFinished))
  (EventDispatchers|BindEventtoJSonCallBack _returnvalue (EventDispatchers|CreateEvent :!event BPAPControllerAutoGenFunc1))
  (EventDispatchers|BindEventtoJSonCallBackType01 _returnvalue (EventDispatchers|CreateEvent :!event BPAPControllerAutoGenFunc))
  (Utilities|FlowControl|Sequence
    (:then_0
      (Class|HTTPObject|ExcuteHttp (Variables|Default|GetBP_HTTPOB) "http://133.186.215.97:51000" "/hierarchy/" "" "" "None"))
    (:then_1
      (Class|HTTPObject|ExcuteHttp (Variables|Default|GetMainHTTP) "http://3.34.116.91:8501" "/api" "/vcmdata" "/getmain" "Type01"))))

(fn ConstructionScript)

(fn BPAPControllerAutoGenFunc1
  (params (Callbackstruct :type Struct%20Array%20Structure))
  (bind (_jsondata _jsondata_type01) (Utilities|Struct|BreakStructArray Callbackstruct))
  (Variables|Default|SetCallbackstruct_1 Callbackstruct)
  (Utilities|FlowControl|Sequence
    (:then_0
      (for _array_element _jsondata
        _)
      (Variables|Default|SetArray%20Element _array_element))
    (:then_1
      (for _array_element_2 _jsondata_type01
        _)
      (return))))

(fn BPAPControllerAutoGenFunc
  (params (Callbackstruct :type Struct%20Array%20Structure))
  (Development|PrintString "Hello")
  (bind _output_get (Variables|Default|SetCallbackstruct Callbackstruct))
  (for _array_element (.JsonData_Type01 (Utilities|Struct|BreakStructArray _output_get))
    (Development|PrintString (.dataName (Utilities|Struct|BreakJsonType01Struct _array_element))))
  (return))