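; BP_CPS_GameMode is a game mode Blueprint that sets the first player controller to Game and UI input with a visible mouse cursor on BeginPlay.
; OnProceess and OnFinished events print transfer progress and success to the screen as debug output, with nothing in the graph binding or calling them.
; A disconnected HUD-to-widget cast chain and an unused BPHTTPOB item reference remain in the graph.
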(event Custom|OnProceess
  (params (RecvSize :type Integer) (TotalSize :type Integer) (Percent :type Float%20%28single-precision%29))
  (Development|PrintString (Utilities|String|ToString(Text) (Utilities|Text|FormatText "{a}/{b} 는 {P}" RecvSize TotalSize Percent)) true true "(R=1.000000,G=0.095008,B=0.000000,A=1.000000)" 1e+01))

(event Custom|OnFinished
  (params (bIsSuccess :type Boolean) (ContentPath :type String))
  (Development|PrintString (Utilities|String|ToString(Boolean) bIsSuccess) true true "(R=1.000000,G=0.076702,B=0.000000,A=1.000000)" 1e+01)
  (Development|PrintString "Hello"))

(event EventBeginPlay
  (bind _returnvalue (Game|GetPlayerController 0))
  (Input|SetInputModeGameandUI _returnvalue 0 "DoNotLock" true false)
  (Variables|/Script/Engine.PlayerController|SetbShowMouseCursor _returnvalue true))

(event EventTick
  (params (DeltaSeconds :type Float%20%28single-precision%29)))

(fn ConstructionScript)